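; BP_HP_Altar is a level altar actor that applies a recovery gameplay effect when called.
; Entering its Box as BP_Character creates a WBP_Altar_UI widget on screen, and leaving removes it.
; CallAltar receives an Ability System Component and applies GE_CharmRecover1 to it through GAS; this graph does not call it itself.
; Disconnected nodes for toggling a Widget component's visibility remain unused.
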(event `self.Box.OnComponentBeginOverlap`
  (params (OverlappedComponent :type "PrimitiveComponent Object Reference") (OtherActor :type "Actor Object Reference") (OtherComp :type "PrimitiveComponent Object Reference") (OtherBodyIndex :type Integer) (bFromSweep :type Boolean) (SweepResult :type "HitResult Structure (by ref)"))
  (cast `/Game/Moonfall/Character/BP_Character` OtherActor)
  (bind _returnvalue (`|CreateWidget` "/Game/Moonfall/Objects/LevelActor/HP_Altar/WBP_Altar_UI.WBP_Altar_UI_C" (`GameplayStatics.GetPlayerController` 0)))
  (bind _output_get (set `self.AltarWidget` _returnvalue))
  (`UserWidget.AddToViewport` _output_get 0))

(event `self.Box.OnComponentEndOverlap`
  (params (OverlappedComponent :type "PrimitiveComponent Object Reference") (OtherActor :type "Actor Object Reference") (OtherComp :type "PrimitiveComponent Object Reference") (OtherBodyIndex :type Integer))
  (cast `/Game/Moonfall/Character/BP_Character` OtherActor)
  (`/Engine/EditorBlueprintResources/StandardMacros.IsValid` (stale `self.Box.OnComponentBeginOverlap` _output_get)
    (:`Is Valid`
      (`Widget.RemoveFromParent` (stale `self.Box.OnComponentBeginOverlap` _output_get)))))

(event `/Game/Moonfall/Objects/LevelActor/HP_Altar/BPI_Altar.CallAltar`
  (params (AbilitySystemComponent :type "GSCAbilitySystemComponent Object Reference"))
  (`/Engine/EditorBlueprintResources/StandardMacros.IsValid` AbilitySystemComponent
    (:`Is Valid`
      (`AbilitySystemComponent.BP_ApplyGameplayEffectToSelf` AbilitySystemComponent "/Game/Moonfall/Objects/LevelActor/HP_Altar/GE_CharmRecover1.GE_CharmRecover1_C" 0.0 (`AbilitySystemComponent.MakeEffectContext` AbilitySystemComponent)))))

(fn `UserConstructionScript`)