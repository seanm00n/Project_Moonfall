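; Projectile actor that deals blade slash damage through the Gameplay Ability System to actors overlapping its Box.
; On overlap it skips the Instigator and applies GE_BladeSlash_Damage to any actor with an Ability System Component.
; The target applies the effect to itself with its own effect context, so the Instigator is not passed as the damage source.
; An IgnoreActor filter loop exists but is unconnected.
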(event `self.Box.OnComponentBeginOverlap`
  (params (OverlappedComponent :type "PrimitiveComponent Object Reference") (OtherActor :type "Actor Object Reference") (OtherComp :type "PrimitiveComponent Object Reference") (OtherBodyIndex :type Integer) (bFromSweep :type Boolean) (SweepResult :type "HitResult Structure (by ref)"))
  (bind _returnvalue (`AbilitySystemBlueprintLibrary.GetAbilitySystemComponent` OtherActor))
  (if (!= OtherActor (`self.Instigator`))
    (`/Engine/EditorBlueprintResources/StandardMacros.IsValid` _returnvalue
      (:`Is Valid`
        (`AbilitySystemComponent.BP_ApplyGameplayEffectToSelf` _returnvalue "/Game/Moonfall/FXActor/GE_BladeSlash_Damage.GE_BladeSlash_Damage_C" 0.0 (`AbilitySystemComponent.MakeEffectContext` _returnvalue))))))

(fn `UserConstructionScript`)