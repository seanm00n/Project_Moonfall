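; Player character for Moonfall melee combat, built on GAS Companion.
; Input events drive attack buffering, blocking, running, altar interaction and dropping held items, while attack, evade and parry snap yaw toward the TargetSystem's lock-on target.
; A DidItHit component traces sword hits through TraceOn/TraceOff, with a toggleable Niagara trail.
; GSCCore events clamp Health, Lotus and Stamina and open a map on death; several combat and interaction test chains are left unwired.
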(event `EnhancedInput|/Game/Moonfall/Character/Ability/Combo1/IA_NormalAttack`
  (params (ActionValue :type Boolean) (ElapsedSeconds :type "Float (double-precision)") (TriggeredSeconds :type "Float (double-precision)") (InputAction :type "InputAction Object Reference" :default "/Game/Moonfall/Character/Ability/Combo1/IA_NormalAttack.IA_NormalAttack"))
  ;[1 1 1] Mouse Left
)

(event `Key|LeftMouseButton`
  (params (Key :type "Key Structure"))
  ;[1 1 1] Mouse Left
)

(event `self.ReceiveBeginPlay`
  ;[1 1 1] BeginPlay
  (bind _asgscuser_widget (cast `GSCUserWidget` (`WidgetComponent.GetUserWidgetObject` (`self.HealthComponent`))))
  (`GSCUserWidget.InitializeWithAbilitySystem` _asgscuser_widget (`self.AbilitySystemComponent`))
  (`SceneComponent.SetHiddenInGame` (`self.NS_SwordTrail`) true false))

(event `CustomEvent`)

(event `EnhancedInput|/Game/Moonfall/Character/Ability/IA_MovementRun`
  (params (ActionValue :type "Vector2D Structure") (ElapsedSeconds :type "Float (double-precision)") (TriggeredSeconds :type "Float (double-precision)") (InputAction :type "InputAction Object Reference" :default "/Game/Moonfall/Character/Ability/IA_MovementRun.IA_MovementRun"))
  (:`Triggered`
    (set `self.isRun` true)))

(event `CustomEvent_1`)

(event `self.ReceiveTick`
  (params (DeltaSeconds :type "Float (single-precision)")))

(event `self.CustomDitItHitActorComponent.OnItemAdded`
  (params (LastItem :type "HitResult Structure"))
  ;[1 1 1] DititHit added
)

(event `self.CombatSystemComponent.OnTakeAttack`
  ;[1 1 1] DititHit added
)

(event `self.SkeletalMesh.OnComponentBeginOverlap`
  (params (OverlappedComponent :type "PrimitiveComponent Object Reference") (OtherActor :type "Actor Object Reference") (OtherComp :type "PrimitiveComponent Object Reference") (OtherBodyIndex :type Integer) (bFromSweep :type Boolean) (SweepResult :type "HitResult Structure (by ref)"))
  ;[1 1 1] DititHit added
  (`KismetSystemLibrary.PrintString` (`KismetStringLibrary.Concat_StrStr` "Classic Collision: " (`KismetSystemLibrary.GetDisplayName` OtherActor)) true true (struct :`G` 0.66 :`B` 1.0 :`A` 1.0) 5.0))

(event `InputAction|AddToInputBuffer`
  (params (Key :type "Key Structure"))
  ;[1 1 1] InputBuffer
  (:`Pressed`
    (`self.AddAttackBuffer` Key)
    (`self.CheckAttackBuffer`)))

(event `EnhancedInput|/Game/Moonfall/Character/Ability/Combo1/IA_NormalAttack`
  (params (ActionValue :type Boolean) (ElapsedSeconds :type "Float (double-precision)") (TriggeredSeconds :type "Float (double-precision)") (InputAction :type "InputAction Object Reference" :default "/Game/Moonfall/Character/Ability/Combo1/IA_NormalAttack.IA_NormalAttack"))
  (bind _returnvalue (`TargetSystemComponent.GetLockedOnTargetActor` (`self.TargetSystem`)))
  (bind (_returnvalue_roll _returnvalue_pitch _returnvalue_yaw) (`KismetMathLibrary.BreakRotator` (`KismetMathLibrary.FindLookAtRotation` (`self.K2_GetActorLocation`) (`self.K2_GetActorLocation` _returnvalue))))
  ;[1 1 1] RotationAction
  (:`Triggered`
    (if (`self.isTargeting`) :!label _label
      (`/Engine/EditorBlueprintResources/StandardMacros.IsValid` _returnvalue
        (:`Is Valid`
          (`self.K2_SetActorRotation` (`KismetMathLibrary.MakeRotator` 0.0 0.0 _returnvalue_yaw) true))))))

(event `EnhancedInput|/Game/Moonfall/Character/Ability/IA_Parrying`
  (params (ActionValue :type Boolean) (ElapsedSeconds :type "Float (double-precision)") (TriggeredSeconds :type "Float (double-precision)") (InputAction :type "InputAction Object Reference" :default "/Game/Moonfall/Character/Ability/IA_Parrying.IA_Parrying"))
  ;[1 1 1] Block
  (:`Triggered`
    (set `self.isBlocking` true :!label _label_2))
  (:`Started`
    (goto _label_2))
  (:`Ongoing`
    (goto _label_2))
  (:`Canceled`
    (set `self.isBlocking` false :!label _label_3)
    (`self.BlockingCancelDispatcher`))
  (:`Completed`
    (goto _label_3)))

(event `EnhancedInput|/Game/Moonfall/Character/Ability/IA_Evade`
  (params (ActionValue :type Boolean) (ElapsedSeconds :type "Float (double-precision)") (TriggeredSeconds :type "Float (double-precision)") (InputAction :type "InputAction Object Reference" :default "/Game/Moonfall/Character/Ability/IA_Evade.IA_Evade"))
  ;[1 1 1] RotationAction
  (:`Triggered`
    (`self.RotateCharacterToCamera`)
    (goto _label)))

(event `EnhancedInput|/Game/Moonfall/Character/Ability/IA_Parrying`
  (params (ActionValue :type Boolean) (ElapsedSeconds :type "Float (double-precision)") (TriggeredSeconds :type "Float (double-precision)") (InputAction :type "InputAction Object Reference" :default "/Game/Moonfall/Character/Ability/IA_Parrying.IA_Parrying"))
  ;[1 1 1] RotationAction
  (:`Triggered`
    (goto _label)))

(event `EnhancedInput|/Game/Moonfall/Character/Ability/IA_F`
  (params (ActionValue :type Boolean) (ElapsedSeconds :type "Float (double-precision)") (TriggeredSeconds :type "Float (double-precision)") (InputAction :type "InputAction Object Reference" :default "/Game/Moonfall/Character/Ability/IA_F.IA_F"))
  (:`Triggered`
    (for _array_element (`PrimitiveComponent.GetOverlappingActors` (`self.Sphere`) "/Game/Moonfall/Objects/LevelActor/HP_Altar/BP_HP_Altar.BP_HP_Altar_C")
      (if (`KismetSystemLibrary.DoesImplementInterface` _array_element "/Game/Moonfall/Objects/LevelActor/HP_Altar/BPI_Altar.BPI_Altar_C")
        (message `/Game/Moonfall/Objects/LevelActor/HP_Altar/BPI_Altar.CallAltar` _array_element (`self.AbilitySystemComponent`))))))

(event `InputAction|Targeting`
  (params (Key :type "Key Structure"))
  (bind _targetsystem (`self.TargetSystem`))
  ;[1 1 1] Targeting
  (:`Pressed`
    (`TargetSystemComponent.TargetActor` _targetsystem)
    (set `self.isTargeting` (`TargetSystemComponent.IsLocked` _targetsystem))))

(event `self.TargetSystem.OnTargetLockedOn`
  (params (TargetActor :type "Actor Object Reference"))
  ;[1 1 1] Targeting
  (`KismetSystemLibrary.PrintString` (`KismetSystemLibrary.GetDisplayName` TargetActor)))

(event `self.TargetSystem.OnTargetLockedOff`
  (params (TargetActor :type "Actor Object Reference"))
  ;[1 1 1] Targeting
  (`KismetSystemLibrary.PrintString` (`KismetSystemLibrary.GetDisplayName` TargetActor)))

(event `InputAction|BulletTimeTestKey`
  (params (Key :type "Key Structure"))
  ;[1 1 1] 블릿타임 Test
)

(event `InputAction|Interaction`
  (params (Key :type "Key Structure"))
  ;[1 1 1] 상호작용
)

(event `self.TrailOn`
  (`SceneComponent.SetHiddenInGame` (`self.NS_SwordTrail`) false false))

(event `InputAction|InteractionCancel`
  (params (Key :type "Key Structure"))
  ;[1 1 1] 상호작용
  (:`Pressed`
    (bind _currenthelditem (`self.CurrentHeldItem`)
      (:`then`
        (bind _asbp_ability_select_actor (cast `/Game/FightingGame/HUD/AbilitySelect/BP_AbilitySelectActor` _currenthelditem))
        (`/Game/FightingGame/HUD/AbilitySelect/BP_AbilitySelectActor.DropItem` _asbp_ability_select_actor)
        (set `self.CurrentHeldItem` null))
      (:`else`))))

(event `self.TrailOff`
  (`SceneComponent.SetHiddenInGame` (`self.NS_SwordTrail`) true false))

(event `Key|MouseScrollUp`
  (params (Key :type "Key Structure"))
  ;[1 1 1] 상호작용
)

(event `Key|MouseScrollDown`
  (params (Key :type "Key Structure"))
  ;[1 1 1] 상호작용
)

(event `self.GSCCore.OnAbilityActivated`
  (params (Ability :type "GameplayAbility Object Reference")))

(event `self.GSCCore.OnAbilityEnded`
  (params (Ability :type "GameplayAbility Object Reference")))

(event `self.GSCCore.OnAbilityCommit`
  (params (Ability :type "GameplayAbility Object Reference")))

(event `self.GSCCore.OnDamage`
  (params (DamageAmount :type "Float (single-precision)") (SourceCharacter :type "Actor Object Reference") (DamageTags :type "GameplayTagContainer Structure (by ref)"))
  (`KismetSystemLibrary.PrintText` (`|FormatText` "{Self} took damage \nDamage Amount: {Damage} \nDamaged by: {SourceActor} \nTags: {Tags}" self DamageAmount SourceCharacter (`BlueprintGameplayTagLibrary.GetDebugStringFromGameplayTagContainer` DamageTags)) true true (struct :`R` 0.854902 :`G` 0.168627 :`B` 0.160784 :`A` 1.0)))

(event `self.GSCCore.OnPostGameplayEffectExecute`
  (params (Attribute :type "GameplayAttribute Structure") (SourceActor :type "Actor Object Reference") (TargetActor :type "Actor Object Reference") (SourceTags :type "GameplayTagContainer Structure (by ref)") (Payload :type "GSCGameplayEffectExecuteData Structure"))
  (bind _gsccore (`self.GSCCore`))
  (bind _gsccore_2 (`self.GSCCore`))
  (bind _gsccore_3 (`self.GSCCore`))
  ;[1 1 1] AttributeClamp
  (`|SwitchGameplayAttribute` Attribute
    (:`Health`
      (`GSCCoreComponent.ClampAttributeValue` _gsccore_3 (struct :`AttributeName` "Health" :`Attribute` "/Script/GASCompanion.GSCAttributeSet:Health" :`AttributeOwner` "/Script/CoreUObject.Class'\"/Script/GASCompanion.GSCAttributeSet\"'") 0.0 (`GSCCoreComponent.GetAttributeValue` _gsccore_3 (struct :`AttributeName` "MaxHealth" :`Attribute` "/Script/GASCompanion.GSCAttributeSet:MaxHealth" :`AttributeOwner` "/Script/CoreUObject.Class'\"/Script/GASCompanion.GSCAttributeSet\"'"))))
    (:`Lotus`
      (`GSCCoreComponent.ClampAttributeValue` _gsccore_2 (struct :`AttributeName` "Lotus" :`Attribute` "/Script/Project_Moonfall.LotusAttributeSet:Lotus" :`AttributeOwner` "/Script/CoreUObject.Class'\"/Script/Project_Moonfall.LotusAttributeSet\"'") 0.0 (`GSCCoreComponent.GetAttributeValue` _gsccore_2 (struct :`AttributeName` "MaxLotus" :`Attribute` "/Script/Project_Moonfall.LotusAttributeSet:MaxLotus" :`AttributeOwner` "/Script/CoreUObject.Class'\"/Script/Project_Moonfall.LotusAttributeSet\"'"))))
    (:`Stamina`
      (`GSCCoreComponent.ClampAttributeValue` _gsccore (struct :`AttributeName` "Stamina" :`Attribute` "/Script/GASCompanion.GSCAttributeSet:Stamina" :`AttributeOwner` "/Script/CoreUObject.Class'\"/Script/GASCompanion.GSCAttributeSet\"'") 0.0 (`GSCCoreComponent.GetAttributeValue` _gsccore (struct :`AttributeName` "MaxStamina" :`Attribute` "/Script/GASCompanion.GSCAttributeSet:MaxStamina" :`AttributeOwner` "/Script/CoreUObject.Class'\"/Script/GASCompanion.GSCAttributeSet\"'"))))))

(event `self.GSCCore.OnDeath`
  (`KismetSystemLibrary.PrintString` "player Death")
  (`GameplayStatics.OpenLevelBySoftObjectPtr` "/Game/FightingGame/ThirdPersonMap_2.ThirdPersonMap_2"))

(fn `CheckLookAt`
  (returns (LookAtActor :type "Actor Object Reference"))
  (locals (Length :type "Float (double-precision)" :default 1000.0))
  (bind _followcamera (`self.FollowCamera`))
  (bind _returnvalue (+ (`SceneComponent.K2_GetComponentLocation` _followcamera) (0.0 0.0 0.0)))
  (bind _outhit (`KismetSystemLibrary.LineTraceSingle` :`Start` _returnvalue :`End` (+ _returnvalue (* (`KismetMathLibrary.GetForwardVector` (`SceneComponent.K2_GetComponentRotation` _followcamera)) (`local.Length`))) :`TraceChannel` "TraceTypeQuery2" :`DrawDebugType` "ForDuration"))
  (if (`KismetSystemLibrary.DoesImplementInterface` (`.HitActor` (`GameplayStatics.BreakHitResult` _outhit)) "/Script/Project_Moonfall.InteractionInterface")
    (if (not (== (`.HitActor` (`GameplayStatics.BreakHitResult` _outhit)) (`self.LookAtActor`)))
      (bind _output_get (set `self.LookAtActor` (`.HitActor` (`GameplayStatics.BreakHitResult` _outhit))))
      (message `InteractionInterface.LookAt` _output_get self)
      (return (`self.LookAtActor`)))
    (else
      (bind _output_get_2 (set `self.LookAtActor` null))
      (return _output_get_2))))

(fn `GetDitItHit`
  (returns (ReturnValue :type "CustomDitItHitActorComponent Object Reference"))
  (return (`self.CustomDitItHitActorComponent`)))

(fn `SetGravityScale`
  (params (`중력 스케일` :type "Float (single-precision)"))
  (set `CharacterMovementComponent.GravityScale` `중력 스케일` (`self.CharacterMovement`)))

(fn `TraceOff`
  (returns (ReturnValue :type "Array of HitResult Structure"))
  (bind _customditithitactorcomponent (`self.CustomDitItHitActorComponent`))
  (`CustomDitItHitActorComponent.ToggleTraceCheck` _customditithitactorcomponent false)
  (`SceneComponent.SetHiddenInGame` (`self.NS_SwordTrail`) true false)
  (return (`CustomDitItHitActorComponent.HitArray` _customditithitactorcomponent)))

(fn `TraceOn`
  (`CustomDitItHitActorComponent.ToggleTraceCheck` (`self.CustomDitItHitActorComponent`) true))

(fn `UserConstructionScript`
  (`CustomDitItHitActorComponent.SetupVariables` (`self.CustomDitItHitActorComponent`) (`self.Sword`) null)
  (`SkinnedMeshComponent.SetLeaderPoseComponent` (`self.OutLine`) (`self.Mesh`) false false))