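; Gameplay ability for the character's aerial sword attack, layered on a parent ability that it calls on activation, commit and end.
; On commit it zeroes the character's gravity scale to suspend it and listens for the Lotus hit gameplay event, which triggers OnCombatReceived.
; On end it removes effects granting the evade-able attack tag, switches off DidItHit trace checks and sets gravity scale back to a fixed value.
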(event `self.K2_CommitExecute`
  (`parent.K2_CommitExecute`)
  (`AbilityTask_WaitGameplayEvent.WaitGameplayEvent` (struct :`TagName` "Event.HitEvent.Lotus") null
    (:`then`
      (bind _asbp_character (cast `/Game/Moonfall/Character/BP_Character` (`self.GetOwningActorFromActorInfo`)))
      (`/Game/Moonfall/Character/BP_Character.SetGravityScale` _asbp_character 0.0))
    (:`EventReceived`
      (`self.OnCombatReceived` (struct)))))

(event `self.K2_ActivateAbility`
  (`parent.K2_ActivateAbility`))

(event `self.K2_OnEndAbility`
  (params (bWasCancelled :type Boolean))
  (`parent.K2_OnEndAbility` bWasCancelled)
  (`self.EndState`)
  (bind _asbp_character (cast `/Game/Moonfall/Character/BP_Character` (`self.GetOwningActorFromActorInfo`)))
  (`/Game/Moonfall/Character/BP_Character.SetGravityScale` _asbp_character 2.0))

(fn `EndState`
  (bind _owneractor (break `GameplayAbilityActorInfo` (`self.GetActorInfo`)))
  (`AbilitySystemComponent.RemoveActiveEffectsWithGrantedTags` (`AbilitySystemBlueprintLibrary.GetAbilitySystemComponent` _owneractor) (struct :`GameplayTags` (struct :`(TagName` "State.Attack.Able.Evade") :`(TagName` "State.Attack.Able.Parrying") :`(TagName` "State.Parrying.Executable.Perfect"))))
  (`CustomDitItHitActorComponent.ToggleTraceCheck` (`CustomDitItHitActorComponent.GetCustomDitItHitActorComponent` _owneractor) false))