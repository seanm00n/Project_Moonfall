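; Tutorial variant of the dodge gameplay ability, which plays a sword dodge montage section chosen from the character's MoveVector.
; Once the montage starts, it fires the tutorial character's evade dispatcher, then unbinds it.
; A perfect-evade gameplay event grants a Lotus effect once, and any montage exit ends the ability, which zeroes MoveVector.
; Camera-relative rotation logic remains in the graph but is disconnected.
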(event `self.K2_CommitExecute`
  (bind (_movevector_x _movevector_y) (`KismetMathLibrary.BreakVector2D` (`FightingCharacter.MoveVector` (`self.As BP Character`))))
  (bind _asbp_character (cast `/Game/Moonfall/Character/BP_Character` (`.OwnerActor` (break `GameplayAbilityActorInfo` (`self.GetActorInfo`)))))
  (set `self.As BP Character` _asbp_character)
  (`GSCTask_PlayMontageWaitForEvent.PlayMontageAndWaitForEvent` "None" "/Game/Moonfall/Character/Ability/Dodge/AM_Sword_Dodge.AM_Sword_Dodge" (struct :`GameplayTags` (struct :`(TagName` "State.Evade.Perfect.Success"))) 1.0 (`KismetStringLibrary.Conv_StringToName` (`KismetStringLibrary.Concat_StrStr` (`KismetStringLibrary.Conv_Int64ToString` (`KismetMathLibrary.Conv_DoubleToInt64` _movevector_x)) (`KismetStringLibrary.Concat_StrStr` "_" (`KismetStringLibrary.Conv_Int64ToString` (`KismetMathLibrary.Conv_DoubleToInt64` _movevector_y)))))
    (:`then`
      (bind _asbp_character_tutorial_ (cast `/Game/Moonfall/Character/BP_Character_Tutorial_` (`self.GetOwningActorFromActorInfo`)))
      (`/Game/Moonfall/Character/BP_Character_Tutorial_.EvadeTutorialDispatcher` _asbp_character_tutorial_)
      (clear `/Game/Moonfall/Character/BP_Character_Tutorial_.EvadeTutorialDispatcher` _asbp_character_tutorial_))
    (:`OnCompleted`
      (`self.K2_EndAbility` :!label _label))
    (:`OnBlendOut`
      (goto _label))
    (:`OnInterrupted`
      (goto _label))
    (:`OnCancelled`
      (goto _label))
    (:`EventReceived`
      (`/Engine/EditorBlueprintResources/StandardMacros.DoOnce` false
        (:`Completed`
          (`self.BP_ApplyGameplayEffectToOwner` "/Game/Moonfall/Effects/GE_GSC_Lotus_1.GE_GSC_Lotus_1_C")
          (`KismetSystemLibrary.PrintString` "Lotus Get"))))))

(event `self.K2_OnEndAbility`
  (params (bWasCancelled :type Boolean))
  (`KismetSystemLibrary.PrintString` "Dodge End")
  (set `FightingCharacter.MoveVector` (0.0 0.0) (`self.As BP Character`)))