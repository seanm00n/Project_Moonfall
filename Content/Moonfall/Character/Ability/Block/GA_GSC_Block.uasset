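; GA_GSC_Block is the gameplay ability for blocking and parrying, ending when blocking is cancelled.
; It applies GE_JustBlock once per activation and replays AM_Blocking's looping section while blocking is held.
; A perfect-parry event applies GE_GSC_Lotus and plays a random parry montage; the normal-parry branch knocks back, though the montage listens only for perfect.
; It also turns toward lock-on targets and carries an uncalled sphere-trace targeting helper.
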(event `self.K2_OnEndAbility`
  (params (bWasCancelled :type Boolean))
  (goto _label_2 :!via `Reset`))

(event `self.K2_CommitExecute`
  (bind _character (`self.Character`))
  (bind _returnvalue (`Actor.K2_GetActorLocation` _character))
  (bind (_returnvalue_x _returnvalue_y) (`KismetMathLibrary.BreakVector` (* (- (`Actor.K2_GetActorLocation` (`.Instigator` (break `GameplayEventData` (`self.Event Data`)))) _returnvalue) -1.0)))
  (bind _returnvalue_2 (`KismetMathLibrary.MakeVector` _returnvalue_x _returnvalue_y))
  (bind _returnvalue_3 (`KismetMathLibrary.Normal` _returnvalue_2))
  (bind _returnvalue_4 (* _returnvalue_3 150.0))
  (bind _asbp_character (cast `/Game/Moonfall/Character/BP_Character` (`.OwnerActor` (break `GameplayAbilityActorInfo` (`self.GetActorInfo`)))))
  (bind _output_get (set `self.Character` _asbp_character))
  (add `/Game/Moonfall/Character/BP_Character.BlockingCancelDispatcher` _output_get (delegate `CheckBlocking`))
  (add `self.OnActivateCombatAbility` (delegate `Targeting`))
  (bind (_asynctaskproxy _eventtag _eventdata) (`GSCTask_PlayMontageWaitForEvent.PlayMontageAndWaitForEvent` "None" "/Game/Moonfall/Character/Ability/Block/AM_Blocking.AM_Blocking" (struct :`GameplayTags` (struct :`(TagName` "State.Parrying.Perfect.Success") :`(TagName` "State.Parrying.Normal.Success"))) 1.0 (`self.StartSection`) :!label _label)
    (:`then`
      (`/Engine/EditorBlueprintResources/StandardMacros.DoOnce` false :!label _label_2
        (:`Completed`
          (`self.BP_ApplyGameplayEffectToOwner` "/Game/Moonfall/Character/Ability/Block/GE_JustBlock.GE_JustBlock_C"))))
    (:`OnCompleted`
      (`self.CheckBlock` :!label _label_3))
    (:`OnBlendOut`
      (goto _label_3))
    (:`OnInterrupted`)
    (:`OnCancelled`)
    (:`EventReceived`
      (set `self.Event Data` _eventdata)
      (`|SwitchGameplayTag` _eventtag
        (:`State.Parrying.Normal.Success`
          (`self.MontageJumpToSection` "BlockBreak")
          (`KismetSystemLibrary.PrintString` "Defense")
          (`KismetSystemLibrary.PrintString` (`KismetStringLibrary.Conv_VectorToString` _returnvalue_2))
          (`KismetSystemLibrary.PrintString` (`KismetStringLibrary.Conv_VectorToString` _returnvalue_3))
          (`CharacterMovementComponent.AddForce` (`Character.CharacterMovement` _character) _returnvalue_4)
          (`Actor.K2_SetActorLocation` _character (+ _returnvalue _returnvalue_4) true false))
        (:`State.Parrying.Perfect.Success`
          (`/Engine/EditorBlueprintResources/StandardMacros.DoOnce` false
            (:`Completed`
              (`KismetSystemLibrary.PrintString` "Defense Perfect")
              (`self.BP_ApplyGameplayEffectToOwner` "/Game/Moonfall/Character/Effects/GE_GSC_Lotus.GE_GSC_Lotus_C")
              (`self.MontageStop` -1.0)
              (`AbilityTask_PlayMontageAndWait.CreatePlayMontageAndWaitProxy` "None" (`KismetArrayLibrary.Array_Random` (`self.JustParryingAM`))
                (:`then`
                  (`KismetSystemLibrary.PrintString` "Hello"))))))))))

(event `CheckBlock`
  (if (`/Game/Moonfall/Character/BP_Character.isBlocking` (`self.Character`))
    (set `self.StartSection` "Blocking")
    (goto _label)
    (else
      (`self.K2_EndAbility`))))

(event `Targeting`
  (bind _character (`self.Character`))
  (bind _returnvalue (`TargetSystemComponent.GetLockedOnTargetActor` (`/Game/Moonfall/Character/BP_Character.TargetSystem` _character)))
  (if (`/Game/Moonfall/Character/BP_Character.isTargeting` _character)
    (`/Engine/EditorBlueprintResources/StandardMacros.IsValid` _returnvalue
      (:`Is Valid`
        (`Actor.K2_SetActorRotation` _character (`KismetMathLibrary.FindLookAtRotation` (`Actor.K2_GetActorLocation` _character) (`Actor.K2_GetActorLocation` _returnvalue)) false)))))

(event `CheckBlocking`
  (`self.K2_EndAbility`))

(fn `GetEndTraceLocation`
  (params (Actor :type "Actor Object Reference"))
  (returns (EndTrace :type "Vector Structure"))
  (return (+ (`self.GetStartTraceLocation` Actor) (* (`Actor.GetActorForwardVector` Actor) (`self.Distance`)))))

(fn `GetStartTraceLocation`
  (params (Actor :type "Actor Object Reference"))
  (returns (StartTrace :type "Vector Structure"))
  (return (`KismetMathLibrary.TransformLocation` (`Actor.GetTransform` Actor) (`self.OffsetFromActor`))))

(fn `GetTargets`
  (params (TargetingActor :type "Actor Object Reference") (EventData :type "GameplayEventData Structure"))
  (returns (OutHitResults :type "Array of HitResult Structure") (OutActors :type "Array of Actor Object Reference"))
  (locals (HitResults :type "Array of HitResult Structure"))
  (bind _outhits (`KismetSystemLibrary.SphereTraceMultiForObjects` (`self.GetStartTraceLocation` TargetingActor) (`self.GetEndTraceLocation` TargetingActor) (`self.Radius`) (`self.ObjectTypes`) false (`|MakeArray` TargetingActor) (`self.Draw Debug`) true (struct :`R` 1.0 :`A` 1.0) (struct :`G` 1.0 :`A` 1.0) 2.0))
  (for _array_element _outhits
    (`/Engine/EditorBlueprintResources/StandardMacros.IsValid` (`.HitActor` (`GameplayStatics.BreakHitResult` _array_element))
      (:`Is Valid`
        (`KismetArrayLibrary.Array_Add` (`local.HitResults`) _array_element))))
  (return (`local.HitResults`)))