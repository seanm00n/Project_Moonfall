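; Target type Blueprint for abilities that gathers hit results with a multi-sphere object trace from the targeting actor.
; The sweep starts at an actor-local offset and extends a set distance along the actor's forward vector, using configurable radius, object types and debug drawing.
; It ignores the targeting actor, prints a debug string and returns hits with valid actors through the HitResults variable, which is not cleared here.
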(fn `GetEndTraceLocation`
  (params (Actor :type "Actor Object Reference"))
  (returns (EndTrace :type "Vector Structure"))
  (return (+ (`self.GetStartTraceLocation` Actor) (* (`Actor.GetActorForwardVector` Actor) (`self.Distance`)))))

(fn `GetStartTraceLocation`
  (params (Actor :type "Actor Object Reference"))
  (returns (StartTrace :type "Vector Structure"))
  (return (`KismetMathLibrary.TransformLocation` (`Actor.GetTransform` Actor) (`self.OffsetFromActor`))))

(fn `GetTargets`
  (params (TargetingActor :type "Actor Object Reference") (EventData :type "GameplayEventData Structure"))
  (returns (OutHitResults :type "Array of HitResult Structure") (OutActors :type "Array of Actor Object Reference"))
  (locals (HitResults :type "Array of HitResult Structure"))
  (bind _targetingactor (`local.TargetingActor`))
  (bind _targetingactor_2 (`local.TargetingActor`))
  (bind _outhits (`KismetSystemLibrary.SphereTraceMultiForObjects` _targetingactor (`self.GetStartTraceLocation` _targetingactor_2) (`self.GetEndTraceLocation` _targetingactor_2) (`self.Radius`) (`self.ObjectTypes`) false (`|MakeArray` (`local.TargetingActor`)) (`self.DrawDebug`) true (struct :`R` 1.0 :`A` 1.0) (struct :`G` 1.0 :`A` 1.0) 2.0))
  (`KismetSystemLibrary.PrintString` _targetingactor "GetTargets")
  (for _array_element _outhits
    (`/Engine/EditorBlueprintResources/StandardMacros.IsValid` (`.HitActor` (`GameplayStatics.BreakHitResult` _array_element))
      (:`Is Valid`
        (`KismetArrayLibrary.Array_Add` (`local.HitResults`) _array_element))))
  (return (`local.HitResults`)))