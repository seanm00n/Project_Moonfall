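; Evade gameplay ability for Moonfall that plays the AM_Evade montage and rewards a successful perfect evade.
; On activation it commits, stops the current montage, then plays the evade montage while listening for the State.Evade.Perfect.Success event.
; That event applies GE_GSC_Lotus to the owner through a DoOnce gate, and any montage finish, blend-out, interruption or cancellation ends the ability.
; The end and activate-from-event handlers only print debug strings.
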(event `self.K2_ActivateAbility`
  (`self.K2_CommitAbility`)
  (`self.MontageStop` -1.0)
  (`GSCTask_PlayMontageWaitForEvent.PlayMontageAndWaitForEvent` "None" "/Game/Moonfall/Character/Ability/Evade/AM_Evade.AM_Evade" (struct :`GameplayTags` (struct :`(TagName` "State.Evade.Perfect.Success")))
    (:`OnCompleted`
      (`self.K2_EndAbility` :!label _label))
    (:`OnBlendOut`
      (goto _label))
    (:`OnInterrupted`
      (goto _label))
    (:`OnCancelled`
      (goto _label))
    (:`EventReceived`
      (`/Engine/EditorBlueprintResources/StandardMacros.DoOnce` false
        (:`Completed`
          (`self.BP_ApplyGameplayEffectToOwner` "/Game/FightingGame/Characters/Effects/GE_GSC_Lotus.GE_GSC_Lotus_C")
          (`KismetSystemLibrary.PrintString` "Lotus Get"))))))

(event `self.K2_OnEndAbility`
  (params (bWasCancelled :type Boolean))
  (`KismetSystemLibrary.PrintString` "Evade End"))

(event `self.K2_ActivateAbilityFromEvent`
  (params (EventData :type "GameplayEventData Structure (by ref)"))
  (`KismetSystemLibrary.PrintString` "FromEvent"))