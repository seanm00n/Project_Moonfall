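; GAS Companion combat ability for the character's Q sword attack.
; On commit it plays the attack montage, forwards Lotus hit events to OnCombatReceived and registers a callback that turns the character toward its locked-on target.
; Ending the ability jumps to BlockEnd, removes evade-window effects and disables DidItHit tracing.
; Sphere-trace targeting and parry/block logic remain as disconnected leftovers that never run.
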(event `self.K2_CommitExecute`
  (add `self.OnActivateCombatAbility` (delegate `TargetingEvent`))
  (bind _asbp_character (cast `/Game/Moonfall/Character/BP_Character` (`.OwnerActor` (break `GameplayAbilityActorInfo` (`self.GetActorInfo`)))))
  (set `self.Character` _asbp_character)
  (`GSCTask_PlayMontageWaitForEvent.PlayMontageAndWaitForEvent` "None" "/Game/Moonfall/Character/Ability/Attack_type5_Q/AM_Sword_Attack_Q.AM_Sword_Attack_Q" (struct :`GameplayTags` (struct :`(TagName` "Event.HitEvent.Lotus")))
    (:`OnCompleted`
      (`self.K2_EndAbility` :!label _label))
    (:`OnBlendOut`
      (goto _label))
    (:`OnInterrupted`
      (goto _label))
    (:`OnCancelled`
      (goto _label))
    (:`EventReceived`
      (`self.OnCombatReceived` (struct)))))

(event `TargetingEvent`
  (bind _character (`self.Character`))
  (bind _returnvalue (`TargetSystemComponent.GetLockedOnTargetActor` (`/Game/Moonfall/Character/BP_Character.TargetSystem` _character)))
  (if (`/Game/Moonfall/Character/BP_Character.isTargeting` _character)
    (`/Engine/EditorBlueprintResources/StandardMacros.IsValid` _returnvalue
      (:`Is Valid`
        (`Actor.K2_SetActorRotation` _character (`KismetMathLibrary.FindLookAtRotation` (`Actor.K2_GetActorLocation` _character) (`Actor.K2_GetActorLocation` _returnvalue)) false)))))

(event `self.K2_OnEndAbility`
  (params (bWasCancelled :type Boolean))
  (`self.MontageJumpToSection` "BlockEnd")
  (`self.EndState`))

(fn `EndState`
  (bind _owneractor (break `GameplayAbilityActorInfo` (`self.GetActorInfo`)))
  (`AbilitySystemComponent.RemoveActiveEffectsWithGrantedTags` (`AbilitySystemBlueprintLibrary.GetAbilitySystemComponent` _owneractor) (struct :`GameplayTags` (struct :`(TagName` "State.Attack.Able.Evade") :`(TagName` "State.Attack.Able.Parrying") :`(TagName` "State.Parrying.Executable.Perfect"))))
  (`CustomDitItHitActorComponent.ToggleTraceCheck` (`CustomDitItHitActorComponent.GetCustomDitItHitActorComponent` _owneractor) false))

(fn `GetEndTraceLocation`
  (params (Actor :type "Actor Object Reference"))
  (returns (EndTrace :type "Vector Structure"))
  (return (+ (`self.GetStartTraceLocation` Actor) (* (`Actor.GetActorForwardVector` Actor) (`self.Distance`)))))

(fn `GetStartTraceLocation`
  (params (Actor :type "Actor Object Reference"))
  (returns (StartTrace :type "Vector Structure"))
  (return (`KismetMathLibrary.TransformLocation` (`Actor.GetTransform` Actor) (`self.OffsetFromActor`))))

(fn `GetTargets`
  (params (TargetingActor :type "Actor Object Reference") (EventData :type "GameplayEventData Structure"))
  (returns (OutHitResults :type "Array of HitResult Structure") (OutActors :type "Array of Actor Object Reference"))
  (locals (HitResults :type "Array of HitResult Structure"))
  (bind _outhits (`KismetSystemLibrary.SphereTraceMultiForObjects` (`self.GetStartTraceLocation` TargetingActor) (`self.GetEndTraceLocation` TargetingActor) (`self.Radius`) (`self.ObjectTypes`) false (`|MakeArray` TargetingActor) (`self.Draw Debug`) true (struct :`R` 1.0 :`A` 1.0) (struct :`G` 1.0 :`A` 1.0) 2.0))
  (for _array_element _outhits
    (`/Engine/EditorBlueprintResources/StandardMacros.IsValid` (`.HitActor` (`GameplayStatics.BreakHitResult` _array_element))
      (:`Is Valid`
        (`KismetArrayLibrary.Array_Add` (`local.HitResults`) _array_element))))
  (return (`local.HitResults`)))