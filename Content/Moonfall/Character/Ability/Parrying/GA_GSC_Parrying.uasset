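; Parry gameplay ability for Moonfall characters that plays AM_Parrying, commits, and applies GE_JustParrying to the owner.
; The montage task listens for the perfect-parry event, which a DoOnce limits to one response until the ability ends.
; That response applies GE_ParryingCollision to the event's instigator and calls an owner effect with no class set.
; A normal-parry branch only prints, and the forward sphere-trace targeting path is disconnected.
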(event `self.K2_ActivateAbility`
  (bind (_asynctaskproxy _eventtag _eventdata) (`GSCTask_PlayMontageWaitForEvent.PlayMontageAndWaitForEvent` "None" "/Game/Moonfall/Character/Ability/Parrying/AM_Parrying.AM_Parrying" (struct :`GameplayTags` (struct :`(TagName` "State.Parrying.Perfect.Success") :`(TagName` "State.Parrying.Normal.Success"))))
    (:`then`
      (`self.K2_CommitAbility`)
      (`self.BP_ApplyGameplayEffectToOwner` "/Game/Moonfall/Character/Ability/Parrying/GE_JustParrying.GE_JustParrying_C"))
    (:`OnCompleted`
      (`self.K2_EndAbility` :!label _label)
      (goto _label_2 :!via `Reset`))
    (:`OnBlendOut`
      (goto _label))
    (:`OnInterrupted`
      (goto _label))
    (:`OnCancelled`
      (goto _label))
    (:`EventReceived`
      (`|SwitchGameplayTag` _eventtag
        (:`State.Parrying.Normal.Success`
          (`KismetSystemLibrary.PrintString` "Defense"))
        (:`State.Parrying.Perfect.Success`
          (`/Engine/EditorBlueprintResources/StandardMacros.DoOnce` false :!label _label_2
            (:`Completed`
              (`KismetSystemLibrary.PrintString` "Defense Perfect")
              (`self.BP_ApplyGameplayEffectToOwner` null)
              (`AbilitySystemComponent.BP_ApplyGameplayEffectToSelf` :`self` (`AbilitySystemBlueprintLibrary.GetAbilitySystemComponent` (`.Instigator` (break `GameplayEventData` _eventdata))) :`GameplayEffectClass` "/Game/Moonfall/Character/Ability/Parrying/GE_ParryingCollision.GE_ParryingCollision_C"))))))))

(event `self.K2_OnEndAbility`
  (params (bWasCancelled :type Boolean)))

(fn `GetEndTraceLocation`
  (params (Actor :type "Actor Object Reference"))
  (returns (EndTrace :type "Vector Structure"))
  (return (+ (`self.GetStartTraceLocation` Actor) (* (`Actor.GetActorForwardVector` Actor) (`self.Distance`)))))

(fn `GetStartTraceLocation`
  (params (Actor :type "Actor Object Reference"))
  (returns (StartTrace :type "Vector Structure"))
  (return (`KismetMathLibrary.TransformLocation` (`Actor.GetTransform` Actor) (`self.OffsetFromActor`))))

(fn `GetTargets`
  (params (TargetingActor :type "Actor Object Reference") (EventData :type "GameplayEventData Structure"))
  (returns (OutHitResults :type "Array of HitResult Structure") (OutActors :type "Array of Actor Object Reference"))
  (locals (HitResults :type "Array of HitResult Structure"))
  (bind _outhits (`KismetSystemLibrary.SphereTraceMultiForObjects` (`self.GetStartTraceLocation` TargetingActor) (`self.GetEndTraceLocation` TargetingActor) (`self.Radius`) (`self.ObjectTypes`) false (`|MakeArray` TargetingActor) (`self.Draw Debug`) true (struct :`R` 1.0 :`A` 1.0) (struct :`G` 1.0 :`A` 1.0) 2.0))
  (for _array_element _outhits
    (`/Engine/EditorBlueprintResources/StandardMacros.IsValid` (`.HitActor` (`GameplayStatics.BreakHitResult` _array_element))
      (:`Is Valid`
        (`KismetArrayLibrary.Array_Add` (`local.HitResults`) _array_element))))
  (return (`local.HitResults`)))