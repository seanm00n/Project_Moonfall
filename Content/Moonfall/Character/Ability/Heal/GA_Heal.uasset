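; GA_Heal is a Gameplay Ability that heals the owning character and consumes a charm on the HUD.
; On activation it commits the ability, checks the avatar is valid, then applies the GE_Heal effect to its owner.
; It then finds every top-level WB_HUD_Character widget and calls RemoveCharm on it directly.
; The ability ends immediately on both success and failure paths.
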(event `self.K2_ActivateAbility`
  (bind _returnvalue (`self.K2_CommitAbility`))
  (if _returnvalue
    (`/Engine/EditorBlueprintResources/StandardMacros.IsValid` (`self.GetAvatarActorFromActorInfo`)
      (:`Is Valid`
        (`self.BP_ApplyGameplayEffectToOwner` "/Game/Moonfall/Character/Ability/Heal/GE_Heal.GE_Heal_C")
        (bind _foundwidgets (`WidgetBlueprintLibrary.GetAllWidgetsOfClass` "/Game/Moonfall/UI/Stage/WB_HUD_Character.WB_HUD_Character_C"))
        (for _array_element _foundwidgets
          (`/Game/Moonfall/UI/Stage/WB_HUD_Character.Remove Charm` _array_element))
        (`self.K2_EndAbility`))
      (:`Is Not Valid`
        (`self.K2_EndAbility`)))
    (else
      (`self.K2_EndAbility`))))

(event `self.K2_OnEndAbility`
  (params (bWasCancelled :type Boolean)))