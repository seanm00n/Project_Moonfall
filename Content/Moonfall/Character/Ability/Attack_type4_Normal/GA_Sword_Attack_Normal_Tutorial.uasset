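; Gameplay ability for the tutorial variant of the normal sword attack, extending its parent ability.
; On commit, it waits for the Lotus hit event, runs OnCombatReceived, then fires the tutorial character's attack dispatcher and unbinds all listeners, making the notification one-shot.
; On end, EndState removes effects granting the evade-able attack tag and switches off DidItHit trace checks.
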(event `self.K2_CommitExecute`
  (`parent.K2_CommitExecute`)
  (`AbilityTask_WaitGameplayEvent.WaitGameplayEvent` (struct :`TagName` "Event.HitEvent.Lotus") null
    (:`EventReceived`
      (`self.OnCombatReceived` (struct))
      (bind _asbp_character_tutorial_ (cast `/Game/Moonfall/Character/BP_Character_Tutorial_` (`self.GetOwningActorFromActorInfo`)))
      (`/Game/Moonfall/Character/BP_Character_Tutorial_.AttackTutorialDispatcher` _asbp_character_tutorial_)
      (clear `/Game/Moonfall/Character/BP_Character_Tutorial_.AttackTutorialDispatcher` _asbp_character_tutorial_))))

(event `self.K2_ActivateAbility`
  (`parent.K2_ActivateAbility`))

(event `self.K2_OnEndAbility`
  (params (bWasCancelled :type Boolean))
  (`parent.K2_OnEndAbility` bWasCancelled)
  (`self.EndState`))

(fn `EndState`
  (bind _owneractor (break `GameplayAbilityActorInfo` (`self.GetActorInfo`)))
  (`AbilitySystemComponent.RemoveActiveEffectsWithGrantedTags` (`AbilitySystemBlueprintLibrary.GetAbilitySystemComponent` _owneractor) (struct :`GameplayTags` (struct :`(TagName` "State.Attack.Able.Evade") :`(TagName` "State.Attack.Able.Parrying") :`(TagName` "State.Parrying.Executable.Perfect"))))
  (`CustomDitItHitActorComponent.ToggleTraceCheck` (`CustomDitItHitActorComponent.GetCustomDitItHitActorComponent` _owneractor) false))