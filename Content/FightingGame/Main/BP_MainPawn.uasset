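; BP_MainPawn is a main pawn in the FightingGame folder that provides mouse-wheel zoom and input hand-off to other actors.
; BeginPlay sets a fixed starting transform with a 90-degree rotation.
; Wheel input steps a clamped ZoomLevel and, short of the limit, moves the pawn forward from the current camera location by a level-scaled distance, in both scroll directions.
; EnableInputToActor and DisableInputToActor swap player-controller input between the pawn and a given actor.
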(event `self.ReceiveBeginPlay`
  (`self.K2_SetActorLocationAndRotation` (0.0 0.0 0.0) (struct :`Yaw` 90.0)))

(event `Key|MouseScrollUp`
  (params (Key :type "Key Structure"))
  (bind _returnvalue (`GameplayStatics.GetPlayerCameraManager` 0))
  ;[1 1 1] Zoom
  (:`Pressed`
    (bind _output_get (set `self.ZoomLevel` (`KismetMathLibrary.Clamp` (+ (`self.ZoomLevel`) 1) 1 20)))
    (if (< _output_get 20)
      (`self.K2_SetActorLocation` (+ (`PlayerCameraManager.GetCameraLocation` _returnvalue) (* (`KismetMathLibrary.GetForwardVector` (`PlayerCameraManager.GetCameraRotation` _returnvalue)) (* (`self.ZoomLevel`) 20)))))))

(event `Key|MouseScrollDown`
  (params (Key :type "Key Structure"))
  (bind _returnvalue (`GameplayStatics.GetPlayerCameraManager` 0))
  ;[1 1 1] Zoom
  (:`Pressed`
    (bind _output_get (set `self.ZoomLevel` (`KismetMathLibrary.Clamp` (- (`self.ZoomLevel`) 1) 1 20)))
    (if (> _output_get 1)
      (`self.K2_SetActorLocation` (+ (`PlayerCameraManager.GetCameraLocation` _returnvalue) (* (`KismetMathLibrary.GetForwardVector` (`PlayerCameraManager.GetCameraRotation` _returnvalue)) (* (`self.ZoomLevel`) 20)))))))

(fn `DisableInputToActor`
  (params (InputStackActor :type "Actor Object Reference"))
  (bind _returnvalue (`GameplayStatics.GetPlayerController` 0))
  (`self.DisableInput` InputStackActor _returnvalue)
  (`self.EnableInput` _returnvalue))

(fn `EnableInputToActor`
  (params (InputStackActor :type "Actor Object Reference"))
  (bind _returnvalue (`GameplayStatics.GetPlayerController` 0))
  (`self.EnableInput` InputStackActor _returnvalue)
  (`self.DisableInput` _returnvalue))

(fn `UserConstructionScript`)