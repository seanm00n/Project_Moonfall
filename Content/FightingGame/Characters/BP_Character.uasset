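; Playable fighting-game character built on GAS Companion, handling evade, target lock, attack input buffering, item interaction and a bullet-time test.
; Attack keys feed buffer functions defined outside these graphs; evade activates an ability and snaps facing to camera yaw.
; DidItHit mesh traces, toggled through TraceOn/TraceOff, apply a combo damage effect to hit actors, while post-effect events clamp Health, Stamina and Lotus.
; A camera line trace selects interactables through InteractionInterface.
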(event `EnhancedInput|/Game/FightingGame/Characters/Ability/Combo1/Combo1InputAction`
  (params (ActionValue :type Boolean) (ElapsedSeconds :type "Float (double-precision)") (TriggeredSeconds :type "Float (double-precision)") (InputAction :type "InputAction Object Reference" :default "/Game/FightingGame/Characters/Ability/Combo1/Combo1InputAction.Combo1InputAction"))
  ;[1 1 1] Mouse Left
)

(event `self.ReceiveBeginPlay`
  ;[1 1 1] Mouse Left
)

(event `Key|LeftMouseButton`
  (params (Key :type "Key Structure"))
  ;[1 1 1] Mouse Left
)

(event `CustomEvent`
  (`AbilitySystemComponent.BP_ApplyGameplayEffectToSelf` (`self.AbilitySystemComponent`) "/Game/FightingGame/Characters/Effects/GE_Attack4.GE_Attack4_C" 0.0 (`AbilitySystemComponent.MakeEffectContext` (`self.AbilitySystemComponent`))))

(event `CustomEvent_1`
  (`AbilitySystemComponent.BP_ApplyGameplayEffectToSelf` (`self.AbilitySystemComponent`) "/Game/FightingGame/Characters/Effects/GE_Attack3.GE_Attack3_C" 0.0 (`AbilitySystemComponent.MakeEffectContext` (`self.AbilitySystemComponent`))))

(event `EnhancedInput|/Game/FightingGame/Characters/Ability/IA_Combo2`
  (params (ActionValue :type Boolean) (ElapsedSeconds :type "Float (double-precision)") (TriggeredSeconds :type "Float (double-precision)") (InputAction :type "InputAction Object Reference" :default "/Game/FightingGame/Characters/Ability/IA_Combo2.IA_Combo2")))

(event `self.CustomDitItHitActorComponent.OnItemAdded`
  (params (LastItem :type "HitResult Structure"))
  (bind (_bblockinghit _binitialoverlap _time _distance _location _impactpoint _normal _impactnormal _physmat _hitactor) (`GameplayStatics.BreakHitResult` LastItem))
  (bind _returnvalue (`AbilitySystemBlueprintLibrary.GetAbilitySystemComponent` _hitactor))
  ;[1 1 1] DititHit added
  (`KismetSystemLibrary.PrintString` (`KismetStringLibrary.Concat_StrStr` "On hit added:" (`KismetSystemLibrary.GetDisplayName` _hitactor)) true true (struct :`G` 0.66 :`B` 1.0 :`A` 1.0) 5.0)
  (`/Engine/EditorBlueprintResources/StandardMacros.IsValid` _returnvalue
    (:`Is Valid`
      (`AbilitySystemComponent.BP_ApplyGameplayEffectToSelf` _returnvalue "/Game/FightingGame/Characters/Ability/Combo1/GE_Combo1_1Damage.GE_Combo1_1Damage_C" 0.0 (`AbilitySystemComponent.MakeEffectContext` _returnvalue)))))

(event `self.SkeletalMesh.OnComponentBeginOverlap`
  (params (OverlappedComponent :type "PrimitiveComponent Object Reference") (OtherActor :type "Actor Object Reference") (OtherComp :type "PrimitiveComponent Object Reference") (OtherBodyIndex :type Integer) (bFromSweep :type Boolean) (SweepResult :type "HitResult Structure (by ref)"))
  (`KismetSystemLibrary.PrintString` (`KismetStringLibrary.Concat_StrStr` "Classic Collision: " (`KismetSystemLibrary.GetDisplayName` OtherActor)) true true (struct :`G` 0.66 :`B` 1.0 :`A` 1.0) 5.0))

(event `EnhancedInput|/Game/FightingGame/Characters/Ability/IA_MovementRun`
  (params (ActionValue :type "Vector2D Structure") (ElapsedSeconds :type "Float (double-precision)") (TriggeredSeconds :type "Float (double-precision)") (InputAction :type "InputAction Object Reference" :default "/Game/FightingGame/Characters/Ability/IA_MovementRun.IA_MovementRun"))
  (:`Triggered`
    (`KismetSystemLibrary.PrintString` "MovementRun")))

(event `InputAction|AddToInputBuffer`
  (params (Key :type "Key Structure"))
  ;[1 1 1] InputBuffer
  (:`Pressed`
    (`self.AddAttackBuffer` Key)
    (`self.CheckAttackBuffer`)))

(event `EnhancedInput|/Game/FightingGame/Characters/Ability/IA_Evade_MoveTo`
  (params (ActionValue :type Boolean) (ElapsedSeconds :type "Float (double-precision)") (TriggeredSeconds :type "Float (double-precision)") (InputAction :type "InputAction Object Reference" :default "/Game/FightingGame/Characters/Ability/IA_Evade_MoveTo.IA_Evade_MoveTo"))
  (:`Triggered`
    (`KismetSystemLibrary.PrintString` "Evade_MoveTo")))

(event `EnhancedInput|/Game/FightingGame/Characters/Ability/IA_Evade`
  (params (ActionValue :type Boolean) (ElapsedSeconds :type "Float (double-precision)") (TriggeredSeconds :type "Float (double-precision)") (InputAction :type "InputAction Object Reference" :default "/Game/FightingGame/Characters/Ability/IA_Evade.IA_Evade"))
  ;[1 1 1] 회피
  (:`Triggered`
    (`GSCCoreComponent.ActivateAbilityByClass` (`self.GSCCore`) "/Game/FightingGame/Characters/Ability/Evade/GA_Evade.GA_Evade_C" true)))

(event `EnhancedInput|/Game/FightingGame/Characters/Ability/IA_Evade`
  (params (ActionValue :type Boolean) (ElapsedSeconds :type "Float (double-precision)") (TriggeredSeconds :type "Float (double-precision)") (InputAction :type "InputAction Object Reference" :default "/Game/FightingGame/Characters/Ability/IA_Evade.IA_Evade"))
  (bind (_returnvalue_roll _returnvalue_pitch _returnvalue_yaw) (`KismetMathLibrary.BreakRotator` (`SceneComponent.K2_GetComponentRotation` (`self.FollowCamera`))))
  (:`Triggered`
    (`self.K2_SetActorRotation` (`KismetMathLibrary.MakeRotator` 0.0 0.0 _returnvalue_yaw) true)))

(event `InputAction|Targeting`
  (params (Key :type "Key Structure"))
  (:`Pressed`
    (`TargetSystemComponent.TargetActor` (`self.TargetSystem`))))

(event `self.TargetSystem.OnTargetLockedOn`
  (params (TargetActor :type "Actor Object Reference"))
  (`KismetSystemLibrary.PrintString` (`KismetSystemLibrary.GetDisplayName` TargetActor)))

(event `EnhancedInput|/Game/FightingGame/Characters/Ability/IA_Parrying`
  (params (ActionValue :type Boolean) (ElapsedSeconds :type "Float (double-precision)") (TriggeredSeconds :type "Float (double-precision)") (InputAction :type "InputAction Object Reference" :default "/Game/FightingGame/Characters/Ability/IA_Parrying.IA_Parrying")))

(event `self.TargetSystem.OnTargetLockedOff`
  (params (TargetActor :type "Actor Object Reference"))
  (`KismetSystemLibrary.PrintString` (`KismetSystemLibrary.GetDisplayName` TargetActor)))

(event `InputAction|BulletTimeTestKey`
  (params (Key :type "Key Structure"))
  ;[1 1 1] 블릿타임 Test
  (:`Pressed`
    (`GameplayStatics.SetGlobalTimeDilation` 0.5)
    (set `self.CustomTimeDilation` 1.0)
    (`KismetSystemLibrary.Delay` 5.0)
    (`GameplayStatics.SetGlobalTimeDilation` 1.0)
    (set `self.CustomTimeDilation` 1.0)))

(event `InputAction|Interaction`
  (params (Key :type "Key Structure"))
  (:`Pressed`
    (`self.CheckLookAt`)
    (bind _lookatactor (`self.LookAtActor`)
      (:`then`
        (message `InteractionInterface.InteractWith` _lookatactor self))
      (:`else`
        (message `InteractionInterface.InteractWith` (`self.CurrentHeldItem`) self)))))

(event `InputAction|InteractionCancel`
  (params (Key :type "Key Structure"))
  (:`Pressed`
    (bind _currenthelditem (`self.CurrentHeldItem`)
      (:`then`
        (bind _asbp_ability_select_actor (cast `/Game/FightingGame/HUD/AbilitySelect/BP_AbilitySelectActor` _currenthelditem))
        (`/Game/FightingGame/HUD/AbilitySelect/BP_AbilitySelectActor.DropItem` _asbp_ability_select_actor)
        (set `self.CurrentHeldItem` null))
      (:`else`))))

(event `Key|MouseScrollUp`
  (params (Key :type "Key Structure")))

(event `Key|MouseScrollDown`
  (params (Key :type "Key Structure")))

(event `self.GSCCore.OnAbilityActivated`
  (params (Ability :type "GameplayAbility Object Reference")))

(event `self.GSCCore.OnAbilityEnded`
  (params (Ability :type "GameplayAbility Object Reference")))

(event `self.GSCCore.OnAbilityCommit`
  (params (Ability :type "GameplayAbility Object Reference")))

(event `self.GSCCore.OnPostGameplayEffectExecute`
  (params (Attribute :type "GameplayAttribute Structure") (SourceActor :type "Actor Object Reference") (TargetActor :type "Actor Object Reference") (SourceTags :type "GameplayTagContainer Structure (by ref)") (Payload :type "GSCGameplayEffectExecuteData Structure"))
  (bind _gsccore (`self.GSCCore`))
  (bind _gsccore_2 (`self.GSCCore`))
  (bind _gsccore_3 (`self.GSCCore`))
  ;[1 1 1] AttributeClamp
  (`|SwitchGameplayAttribute` Attribute
    (:`Health`
      (`GSCCoreComponent.ClampAttributeValue` _gsccore_3 (struct :`AttributeName` "Health" :`Attribute` "/Script/GASCompanion.GSCAttributeSet:Health" :`AttributeOwner` "/Script/CoreUObject.Class'\"/Script/GASCompanion.GSCAttributeSet\"'") 0.0 (`GSCCoreComponent.GetAttributeValue` _gsccore_3 (struct :`AttributeName` "MaxHealth" :`Attribute` "/Script/GASCompanion.GSCAttributeSet:MaxHealth" :`AttributeOwner` "/Script/CoreUObject.Class'\"/Script/GASCompanion.GSCAttributeSet\"'"))))
    (:`Lotus`
      (`GSCCoreComponent.ClampAttributeValue` _gsccore_2 (struct :`AttributeName` "Lotus" :`Attribute` "/Script/Project_Moonfall.LotusAttributeSet:Lotus" :`AttributeOwner` "/Script/CoreUObject.Class'\"/Script/Project_Moonfall.LotusAttributeSet\"'") 0.0 (`GSCCoreComponent.GetAttributeValue` _gsccore_2 (struct :`AttributeName` "MaxLotus" :`Attribute` "/Script/Project_Moonfall.LotusAttributeSet:MaxLotus" :`AttributeOwner` "/Script/CoreUObject.Class'\"/Script/Project_Moonfall.LotusAttributeSet\"'"))))
    (:`Stamina`
      (`GSCCoreComponent.ClampAttributeValue` _gsccore (struct :`AttributeName` "Stamina" :`Attribute` "/Script/GASCompanion.GSCAttributeSet:Stamina" :`AttributeOwner` "/Script/CoreUObject.Class'\"/Script/GASCompanion.GSCAttributeSet\"'") 0.0 (`GSCCoreComponent.GetAttributeValue` _gsccore (struct :`AttributeName` "MaxStamina" :`Attribute` "/Script/GASCompanion.GSCAttributeSet:MaxStamina" :`AttributeOwner` "/Script/CoreUObject.Class'\"/Script/GASCompanion.GSCAttributeSet\"'"))))))

(fn `CheckLookAt`
  (returns (LookAtActor :type "Actor Object Reference"))
  (locals (Length :type "Float (double-precision)" :default 1000.0))
  (bind _followcamera (`self.FollowCamera`))
  (bind _returnvalue (+ (`SceneComponent.K2_GetComponentLocation` _followcamera) (0.0 0.0 0.0)))
  (bind _outhit (`KismetSystemLibrary.LineTraceSingle` :`Start` _returnvalue :`End` (+ _returnvalue (* (`KismetMathLibrary.GetForwardVector` (`SceneComponent.K2_GetComponentRotation` _followcamera)) (`local.Length`))) :`TraceChannel` "TraceTypeQuery2" :`DrawDebugType` "ForDuration"))
  (if (`KismetSystemLibrary.DoesImplementInterface` (`.HitActor` (`GameplayStatics.BreakHitResult` _outhit)) "/Script/Project_Moonfall.InteractionInterface")
    (if (not (== (`.HitActor` (`GameplayStatics.BreakHitResult` _outhit)) (`self.LookAtActor`)))
      (bind _output_get (set `self.LookAtActor` (`.HitActor` (`GameplayStatics.BreakHitResult` _outhit))))
      (message `InteractionInterface.LookAt` _output_get self)
      (return (`self.LookAtActor`)))
    (else
      (bind _output_get_2 (set `self.LookAtActor` null))
      (return _output_get_2))))

(fn `GetDitItHit`
  (returns (ReturnValue :type "CustomDitItHitActorComponent Object Reference"))
  (return (`self.CustomDitItHitActorComponent`)))

(fn `TraceOff`
  (returns (HitResults :type "Array of HitResult Structure"))
  (bind _customditithitactorcomponent (`self.CustomDitItHitActorComponent`))
  (`CustomDitItHitActorComponent.ToggleTraceCheck` _customditithitactorcomponent false)
  (return (`CustomDitItHitActorComponent.HitArray` _customditithitactorcomponent)))

(fn `TraceOn`
  (`CustomDitItHitActorComponent.ToggleTraceCheck` (`self.CustomDitItHitActorComponent`) true)
  (return))

(fn `UserConstructionScript`
  (`CustomDitItHitActorComponent.SetupVariables` (`self.CustomDitItHitActorComponent`) (`self.SkeletalMesh`) null))