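; Inspectable, holdable actor in the ability-select HUD folder that snaps to the BP_AbilitySelector's SkillSelect on BeginPlay.
; InteractWith picks it up into BP_Character's ItemGrip, or starts inspection if an item is already held.
; Inspection moves input from player to actor and places it before the camera for left-drag rotation and wheel zoom; Interaction ends it.
; DropItem detaches it and restores physics; LookAt is empty.
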(event `self.ReceiveBeginPlay`
  (bind _returnvalue (`GameplayStatics.GetActorOfClass` "/Game/FightingGame/HUD/AbilitySelect/BP_AbilitySelector.BP_AbilitySelector_C"))
  (bind _skillselect (`/Game/FightingGame/HUD/AbilitySelect/BP_AbilitySelector.SkillSelect` _returnvalue)
    (:`then`
      (`self.K2_AttachToComponent` _skillselect "None" "SnapToTarget" "SnapToTarget" "KeepRelative"))
    (:`else`)))

(event `InputAxisKey|MouseX`
  (params (AxisValue :type "Float (single-precision)"))
  (if (`self.isRotating`)
    (`self.K2_SetActorRotation` (`KismetMathLibrary.ComposeRotators` (`self.K2_GetActorRotation`) (`KismetMathLibrary.MakeRotator` 0.0 0.0 (* AxisValue -5.0))))))

(event `Key|LeftMouseButton`
  (params (Key :type "Key Structure"))
  (:`Pressed`
    (set `self.isRotating` true))
  (:`Released`
    (set `self.isRotating` false)))

(event `InputAxisKey|MouseY`
  (params (AxisValue :type "Float (single-precision)"))
  (if (`self.isRotating`)
    (`self.K2_SetActorRotation` (`KismetMathLibrary.ComposeRotators` (`self.K2_GetActorRotation`) (`KismetMathLibrary.MakeRotator` 0.0 (* AxisValue -5.0))))))

(event `Key|MouseScrollUp`
  (params (Key :type "Key Structure"))
  (bind _returnvalue (`GameplayStatics.GetPlayerCameraManager` 0))
  (:`Pressed`
    (bind _output_get (set `self.ZoomLevel` (`KismetMathLibrary.Clamp` (+ (`self.ZoomLevel`) 1) 1 20)))
    (if (< _output_get 20)
      (`self.K2_SetActorLocation` (+ (`PlayerCameraManager.GetCameraLocation` _returnvalue) (* (`KismetMathLibrary.GetForwardVector` (`PlayerCameraManager.GetCameraRotation` _returnvalue)) (* (`self.ZoomLevel`) 20)))))))

(event `Key|MouseScrollDown`
  (params (Key :type "Key Structure"))
  (bind _returnvalue (`GameplayStatics.GetPlayerCameraManager` 0))
  (:`Pressed`
    (bind _output_get (set `self.ZoomLevel` (`KismetMathLibrary.Clamp` (- (`self.ZoomLevel`) 1) 1 20)))
    (if (> _output_get 1)
      (`self.K2_SetActorLocation` (+ (`PlayerCameraManager.GetCameraLocation` _returnvalue) (* (`KismetMathLibrary.GetForwardVector` (`PlayerCameraManager.GetCameraRotation` _returnvalue)) (* (`self.ZoomLevel`) 20)))))))

(event `InputAction|Interaction`
  (params (Key :type "Key Structure"))
  (:`Pressed`
    (`self.StopInspect`)))

(fn `DropItem`
  (bind _returnvalue (`GameplayStatics.GetPlayerCameraManager` 0))
  (bind _staticmesh (`self.StaticMesh`))
  (`self.K2_DetachFromActor` "KeepWorld" "KeepWorld" "KeepWorld")
  (`self.K2_SetActorLocation` (+ (`PlayerCameraManager.GetCameraLocation` _returnvalue) (* (`KismetMathLibrary.GetForwardVector` (`PlayerCameraManager.GetCameraRotation` _returnvalue)) 600.0)))
  (`PrimitiveComponent.SetSimulatePhysics` _staticmesh true)
  (`PrimitiveComponent.SetCollisionEnabled` _staticmesh "QueryAndPhysics"))

(fn `InteractWith`
  (params (Player :type "Character Object Reference"))
  (bind _output_get (set `self.SkillSelect` Player))
  (bind _asbp_character (cast `/Game/Moonfall/Character/BP_Character` _output_get))
  (`/Game/Moonfall/Character/BP_Character.CurrentHeldItem` _asbp_character
    (:`then`
      (`self.StartInspect`))
    (:`else`
      (`self.PickUpItem`))))

(fn `LookAt`
  (params (Player :type "Character Object Reference")))

(fn `PickUpItem`
  (bind _asbp_character (cast `/Game/Moonfall/Character/BP_Character` (`self.SkillSelect`)))
  (`self.K2_AttachToComponent` (`/Game/Moonfall/Character/BP_Character.ItemGrip` _asbp_character) "None" "SnapToTarget" "SnapToTarget" "KeepRelative")
  (`PrimitiveComponent.SetSimulatePhysics` (`self.StaticMesh`) false)
  (`PrimitiveComponent.SetCollisionEnabled` (`self.StaticMesh`) "NoCollision")
  (bind _asbp_character_2 (cast `/Game/Moonfall/Character/BP_Character` (`self.SkillSelect`)))
  (set `/Game/Moonfall/Character/BP_Character.CurrentHeldItem` self _asbp_character_2))

(fn `StartInspect`
  (bind _returnvalue (`GameplayStatics.GetPlayerController` 0))
  (bind _returnvalue_2 (`GameplayStatics.GetPlayerCameraManager` 0))
  (`self.DisableInput` (`self.SkillSelect`) _returnvalue)
  (`self.EnableInput` _returnvalue)
  (`self.K2_SetActorLocation` (+ (`PlayerCameraManager.GetCameraLocation` _returnvalue_2) (* (`KismetMathLibrary.GetForwardVector` (`PlayerCameraManager.GetCameraRotation` _returnvalue_2)) 1000.0))))

(fn `StopInspect`
  (bind _returnvalue (`GameplayStatics.GetPlayerController` 0))
  (`self.DisableInput` _returnvalue)
  (`self.EnableInput` (`self.SkillSelect`) _returnvalue)
  (`self.K2_SetActorRelativeLocation` (0.0 0.0 0.0))
  (`self.K2_SetActorRelativeRotation` (struct)))

(fn `UserConstructionScript`)