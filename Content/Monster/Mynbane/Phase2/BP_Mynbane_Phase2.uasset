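; Phase 2 Mynbane boss character, built on the Gameplay Ability System with a boss health bar created at BeginPlay.
; Damage events add to a GSCCore attribute, which Tick prints for debugging.
; Death stops montage and AI logic, sets Blackboard state, hides the boss, disables player input, plays the death sequence and starts dialog via a spawned trigger.
; Construction prepares Bat hit tracing, initially off, and makes the outline mesh follow the main mesh's pose.
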(event `self.ReceiveTick`
  (params (DeltaSeconds :type "Float (single-precision)"))
  (`KismetSystemLibrary.PrintString` (`KismetStringLibrary.Conv_DoubleToString` (`GSCCoreComponent.GetAttributeValue` (`self.GSCCoreComponent`) (struct :`AttributeName` "Stack" :`Attribute` "/Script/Project_Moonfall.MonsterAttributeSet:Stack" :`AttributeOwner` "/Script/CoreUObject.Class'\"/Script/Project_Moonfall.MonsterAttributeSet\"'")))))

(event `self.GSCCoreComponent.OnDamage`
  (params (DamageAmount :type "Float (single-precision)") (SourceCharacter :type "Actor Object Reference") (DamageTags :type "GameplayTagContainer Structure (by ref)"))
  (bind _gsccorecomponent (`self.GSCCoreComponent`))
  ;[1 1 1] OnDamages
  (`GSCCoreComponent.SetAttributeValue` _gsccorecomponent (struct :`AttributeName` "HealthPoint" :`Attribute` "/Script/Project_Moonfall.MonsterAttributeSet:HealthPoint" :`AttributeOwner` "/Script/CoreUObject.Class'\"/Script/Project_Moonfall.MonsterAttributeSet\"'") (+ DamageAmount (`GSCCoreComponent.GetAttributeValue` _gsccorecomponent (struct :`AttributeName` "HealthPoint" :`Attribute` "/Script/Project_Moonfall.MonsterAttributeSet:HealthPoint" :`AttributeOwner` "/Script/CoreUObject.Class'\"/Script/Project_Moonfall.MonsterAttributeSet\"'")))))

(event `self.ReceiveBeginPlay`
  ;[1 1 1] BeginPlay
  (bind _returnvalue (`|CreateWidget` "/Game/Moonfall/UI/WB_BossHealthBar.WB_BossHealthBar_C"))
  (`UserWidget.AddToViewport` _returnvalue 0)
  (`GSCUserWidget.InitializeWithAbilitySystem` _returnvalue (`self.AbilitySystemComponent`))
  (set `TextBlock.Text` "오니" (`/Game/Moonfall/UI/WB_BossHealthBar.MonsterName` _returnvalue)))

(event `self.GSCCoreComponent.OnDeath`
  ;[1 1 1] OnDeath
  (`self.StopAnimMontage` null)
  (`BrainComponent.StopLogic` (`AIController.BrainComponent` (`AIBlueprintHelperLibrary.GetAIController` self)) "Death")
  (`BlackboardComponent.SetValueAsEnum` (`AIController.Blackboard` (`AIBlueprintHelperLibrary.GetAIController` self)) (`self.State`) 3)
  (`self.SetActorHiddenInGame` true)
  (`self.DisableInput` (`GameplayStatics.GetPlayerCharacter` 0) (`GameplayStatics.GetPlayerController` 0))
  (bind (_outactor _returnvalue) (`LevelSequencePlayer.CreateLevelSequencePlayer` "/Game/Cinematics/sohyeon/Boss2_die.Boss2_die"))
  (`MovieSceneSequencePlayer.Play` _returnvalue)
  (bind _returnvalue_2 (`|SpawnActorFromClass` "/Game/Moonfall/UI/Dialog/Stage_2/BP_Trigger_Dialog_Input_S_6_1.BP_Trigger_Dialog_Input_S_6_1_C" (`self.GetTransform` (`GameplayStatics.GetPlayerCharacter` 0)) "Undefined" "OverrideRootScale" null false null))
  (`/Game/Moonfall/UI/Dialog/BP_Trigger_Dialog_Input.StartDialog` _returnvalue_2))

(fn `Update Walk Speed`
  (params (MaxWalkSpeed :type "Float (single-precision)"))
  (set `CharacterMovementComponent.MaxWalkSpeed` MaxWalkSpeed (`self.CharacterMovement`)))

(fn `UserConstructionScript`
  (bind _customditithitactorcomponent (`self.CustomDitItHitActorComponent`))
  (`CustomDitItHitActorComponent.SetupVariables` _customditithitactorcomponent (`self.Bat`) null)
  (`CustomDitItHitActorComponent.ToggleTraceCheck` _customditithitactorcomponent false)
  (`SkinnedMeshComponent.SetLeaderPoseComponent` (`self.MeshOutline`) (`self.Mesh`) false false))