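; Phase 1 Mynbane monster character, built on GAS Companion with an ability-system-bound health widget and a walk speed setter.
; Damage events add the amount to a GSC attribute, whose value is debug-printed every tick.
; Death stops AI logic, sets the blackboard state, plays the death montage and destroys the actor after a short delay.
; Construction enables DidItHit hit tracing on the skeletal mesh.
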(event `self.ReceiveTick`
  (params (DeltaSeconds :type "Float (single-precision)"))
  (`KismetSystemLibrary.PrintString` (`KismetStringLibrary.Conv_DoubleToString` (`GSCCoreComponent.GetAttributeValue` (`self.GSCCoreComponent`) (struct :`AttributeName` "Stack" :`Attribute` "/Script/Project_Moonfall.MonsterAttributeSet:Stack" :`AttributeOwner` "/Script/CoreUObject.Class'\"/Script/Project_Moonfall.MonsterAttributeSet\"'")))))

(event `self.GSCCoreComponent.OnDamage`
  (params (DamageAmount :type "Float (single-precision)") (SourceCharacter :type "Actor Object Reference") (DamageTags :type "GameplayTagContainer Structure (by ref)"))
  (bind _gsccorecomponent (`self.GSCCoreComponent`))
  ;[1 1 1] OnDamages
  (`GSCCoreComponent.SetAttributeValue` _gsccorecomponent (struct :`AttributeName` "HealthPoint" :`Attribute` "/Script/Project_Moonfall.MonsterAttributeSet:HealthPoint" :`AttributeOwner` "/Script/CoreUObject.Class'\"/Script/Project_Moonfall.MonsterAttributeSet\"'") (+ DamageAmount (`GSCCoreComponent.GetAttributeValue` _gsccorecomponent (struct :`AttributeName` "HealthPoint" :`Attribute` "/Script/Project_Moonfall.MonsterAttributeSet:HealthPoint" :`AttributeOwner` "/Script/CoreUObject.Class'\"/Script/Project_Moonfall.MonsterAttributeSet\"'")))))

(event `self.ReceiveBeginPlay`
  ;[1 1 1] BeginPlay
  (bind _asgscuser_widget (cast `GSCUserWidget` (`WidgetComponent.GetUserWidgetObject` (`self.HealthComponent`))))
  (`GSCUserWidget.InitializeWithAbilitySystem` _asgscuser_widget (`self.AbilitySystemComponent`)))

(event `self.GSCCoreComponent.OnDeath`
  ;[1 1 1] OnDeath
  (`self.StopAnimMontage` null)
  (`BrainComponent.StopLogic` (`AIController.BrainComponent` (`AIBlueprintHelperLibrary.GetAIController` self)) "Death")
  (`BlackboardComponent.SetValueAsEnum` (`AIController.Blackboard` (`AIBlueprintHelperLibrary.GetAIController` self)) (`self.State`) 3)
  (`|PlayMontage` (`self.Mesh`) "/Game/Monster/Mynbane/Anim/Montage/reAnim_Die_Montage.reAnim_Die_Montage" ; Death
    (:`then`
      _)
    (:`OnCompleted`
      _)
    (:`OnBlendOut`
      _)
    (:`OnInterrupted`
      _))
  (`KismetSystemLibrary.Delay` 2.0)
  (`self.K2_DestroyActor`)
  (`KismetSystemLibrary.PrintString` "Darknessy::Death"))

(fn `Update Walk Speed`
  (params (MaxWalkSpeed :type "Float (single-precision)"))
  (set `CharacterMovementComponent.MaxWalkSpeed` MaxWalkSpeed (`self.CharacterMovement`)))

(fn `UserConstructionScript`
  (bind _customditithitactorcomponent (`self.CustomDitItHitActorComponent`))
  (`CustomDitItHitActorComponent.SetupVariables` _customditithitactorcomponent (`self.SkeletalMesh`) null)
  (`CustomDitItHitActorComponent.ToggleTraceCheck` _customditithitactorcomponent true))