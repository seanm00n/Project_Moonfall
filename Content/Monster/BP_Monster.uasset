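; BP_Monster is a monster character Blueprint that exposes helper functions for movement, position and health.
; It sets the CharacterMovement max walk speed from a parameter and returns the actor's location.
; ModHP adds its Damage argument to HealthPoint, so damage must be negative to reduce health, and CheckDeath reports true once HealthPoint is zero or below.
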(fn `CheckDeath`
  (returns (IsDeath :type Boolean))
  (if (<= (`self.HealthPoint`) 0.0)
    (return true)
    (else
      (return false))))

(fn `GetPosition`
  (returns (ReturnValue :type "Vector Structure"))
  (return (`self.K2_GetActorLocation`)))

(fn `ModHP`
  (params (Damage :type "Float (double-precision)"))
  (set `self.HealthPoint` (+ Damage (`self.HealthPoint`))))

(fn `Update Walk Speed`
  (params (`최대 걷기 속도` :type "Float (single-precision)"))
  (set `CharacterMovementComponent.MaxWalkSpeed` `최대 걷기 속도` (`self.CharacterMovement`)))

(fn `UserConstructionScript`)