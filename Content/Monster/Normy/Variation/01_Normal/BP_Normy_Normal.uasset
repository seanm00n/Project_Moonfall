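; Normal variant of the Normy monster, shown to the player as "외눈박이", with melee-style hit tracing and death handling.
; On BeginPlay it stores its start position in the Blackboard and creates a boss health bar bound to its ability system, with the numeric text hidden.
; Construction points the DidItHit component at the skeletal mesh with tracing off and makes the outline mesh follow the main pose.
; GSCCore death destroys the actor; helpers set walk speed and return the start position.
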(event `self.ReceiveBeginPlay`
  (bind _output_get (set `self.StartPosition` (`self.K2_GetActorLocation`)))
  (`BlackboardComponent.SetValueAsVector` (`AIBlueprintHelperLibrary.GetBlackboard` null) (`self.K_StartPosition`) _output_get)
  (bind _returnvalue (`|CreateWidget` "/Game/Moonfall/UI/WB_BossHealthBar.WB_BossHealthBar_C"))
  (`UserWidget.AddToViewport` _returnvalue 0)
  (`GSCUserWidget.InitializeWithAbilitySystem` _returnvalue (`self.AbilitySystemComponent`))
  (set `TextBlock.Text` "외눈박이" (`/Game/Moonfall/UI/WB_BossHealthBar.MonsterName` _returnvalue))
  (`Widget.SetVisibility` (`/Game/Moonfall/UI/WB_BossHealthBar.HealthText` _returnvalue) "Hidden"))

(event `self.GSCCoreComponent.OnDeath`
  (`self.K2_DestroyActor`))

(fn `GetStartPosition`
  (returns (StartPosition :type "Vector Structure"))
  (return (`self.StartPosition`)))

(fn `Update Walk Speed`
  (params (`최대 걷기 속도` :type "Float (single-precision)"))
  (set `CharacterMovementComponent.MaxWalkSpeed` `최대 걷기 속도` (`self.CharacterMovement`)))

(fn `UserConstructionScript`
  (bind _customditithitactorcomponent (`self.CustomDitItHitActorComponent`))
  (`CustomDitItHitActorComponent.SetupVariables` _customditithitactorcomponent (`self.SkeletalMesh`) null)
  (`CustomDitItHitActorComponent.ToggleTraceCheck` _customditithitactorcomponent false)
  (`SkinnedMeshComponent.SetLeaderPoseComponent` (`self.Outline`) (`self.Mesh`) false false))