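; BP_Normy_3 is a Normy monster character Blueprint that supplies movement and home-position data for its AI.
; The Construction Script binds a DidItHit-style trace component to the skeletal mesh, enables its trace check, and saves the actor's location as StartPosition in a variable and the Blackboard.
; Helper functions set the CharacterMovement max walk speed and return the start position.
; BeginPlay is empty, with a note questioning whether health component and widget are needed.
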(event `self.ReceiveBeginPlay`)

(fn `GetStartPosition`
  (returns (StartPosition :type "Vector Structure"))
  (return (`self.StartPosition`)))

(fn `Update Walk Speed`
  (params (`최대 걷기 속도` :type "Float (single-precision)"))
  (set `CharacterMovementComponent.MaxWalkSpeed` `최대 걷기 속도` (`self.CharacterMovement`)))

(fn `UserConstructionScript`
  (bind _customditithitactorcomponent (`self.CustomDitItHitActorComponent`))
  (`CustomDitItHitActorComponent.SetupVariables` _customditithitactorcomponent (`self.SkeletalMesh`) null)
  (`CustomDitItHitActorComponent.ToggleTraceCheck` _customditithitactorcomponent true)
  (bind _output_get (set `self.StartPosition` (`self.K2_GetActorLocation`)))
  (`BlackboardComponent.SetValueAsVector` (`AIBlueprintHelperLibrary.GetBlackboard` null) (`self.K_StartPosition`) _output_get))