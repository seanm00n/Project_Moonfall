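; BP_Normy is the Normy monster Blueprint, exposing the state and helper functions of an enemy character.
; The construction script records the actor's location as StartPosition, readable through a getter alongside current position, health and attack points.
; AdjHP adds a signed value to health without clamping, and UpdateWalkSpeed sets the movement component's max walk speed.
; GetDistance measures the range from the first player's character to this monster.
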(fn `AdjHP`
  (params (Value :type "Float (double-precision)"))
  (set `self.HealthPoint` (+ Value (`self.HealthPoint`))))

(fn `GetAP`
  (returns (AttackPoint :type "Float (double-precision)"))
  (return (`self.AttackPoint`)))

(fn `GetDistance`
  (returns (distance :type "Float (single-precision)"))
  (return (`self.GetDistanceTo` (`GameplayStatics.GetPlayerCharacter` 0) self)))

(fn `GetHP`
  (returns (HealthPoint :type "Float (double-precision)"))
  (return (`self.HealthPoint`)))

(fn `GetPosition`
  (returns (ReturnValue :type "Vector Structure"))
  (return (`self.K2_GetActorLocation`)))

(fn `GetStartPosition`
  (returns (StartPosition :type "Vector Structure"))
  (return (`self.StartPosition`)))

(fn `Update Walk Speed`
  (params (`최대 걷기 속도` :type "Float (single-precision)"))
  (set `CharacterMovementComponent.MaxWalkSpeed` `최대 걷기 속도` (`self.CharacterMovement`)))

(fn `UserConstructionScript`
  (set `self.StartPosition` (`self.K2_GetActorLocation`)))