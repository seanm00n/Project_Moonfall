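; Darknessy monster character Blueprint that handles hit reactions, phase switching and death.
; AnyDamage compares Damage plus HealthPoint (never written back) to thresholds, enabling Phase2, then at zero or below playing a death montage and destroying the actor after a delay.
; The construction script sets both phase flags true, with Phase2 marked temporary, and a helper function sets maximum walk speed.
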(event `self.ReceiveAnyDamage`
  (params (Damage :type "Float (single-precision)") (DamageType :type "DamageType Object Reference") (InstigatedBy :type "Controller Object Reference") (DamageCauser :type "Actor Object Reference"))
  (bind _returnvalue (+ Damage (`self.HealthPoint`)))
  (`KismetSystemLibrary.PrintString` "Darknessy::Hit")
  (if (<= _returnvalue 75.0)
    (set `self.Phase2` true)
    (if (<= _returnvalue 0.0)
      (`|PlayMontage` null "/Game/Monster/Darknessy/Anim/Hit_Death_Seq_Montage.Hit_Death_Seq_Montage" ; Death
        (:`OnCompleted`
          (`KismetSystemLibrary.Delay` 1.0)
          (`self.K2_DestroyActor`))))))

(fn `Update Walk Speed`
  (params (`최대 걷기 속도` :type "Float (single-precision)"))
  (set `CharacterMovementComponent.MaxWalkSpeed` `최대 걷기 속도` (`self.CharacterMovement`)))

(fn `UserConstructionScript`
  (set `self.Phase1` true)
  (set `self.Phase2` true) ; tmp
)