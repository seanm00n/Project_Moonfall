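; Darknessy phase 1 boss character, built on GAS Companion with a health widget bound to its ability system.
; On damage it adjusts an attribute and, at a low threshold, resets it and prints a Phase2 debug message.
; On death it stops AI logic, sets the blackboard State, plays a death montage and destroys itself after a delay.
; Construction enables DidItHit tracing on the skeletal mesh; a helper sets walk speed.
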(event `self.GSCCoreComponent.OnDamage`
  (params (DamageAmount :type "Float (single-precision)") (SourceCharacter :type "Actor Object Reference") (DamageTags :type "GameplayTagContainer Structure (by ref)"))
  (bind _gsccorecomponent (`self.GSCCoreComponent`))
  (bind _returnvalue (+ DamageAmount (`GSCCoreComponent.GetAttributeValue` _gsccorecomponent (struct :`AttributeName` "HealthPoint" :`Attribute` "/Script/Project_Moonfall.MonsterAttributeSet:HealthPoint" :`AttributeOwner` "/Script/CoreUObject.Class'\"/Script/Project_Moonfall.MonsterAttributeSet\"'"))))
  ;[1 1 1] OnDamages
  (`GSCCoreComponent.SetAttributeValue` _gsccorecomponent (struct :`AttributeName` "HealthPoint" :`Attribute` "/Script/Project_Moonfall.MonsterAttributeSet:HealthPoint" :`AttributeOwner` "/Script/CoreUObject.Class'\"/Script/Project_Moonfall.MonsterAttributeSet\"'") _returnvalue)
  (if (<= _returnvalue 100.0)
    (`GSCCoreComponent.SetAttributeValue` _gsccorecomponent (struct :`AttributeName` "Phase" :`Attribute` "/Script/Project_Moonfall.MonsterAttributeSet:Phase" :`AttributeOwner` "/Script/CoreUObject.Class'\"/Script/Project_Moonfall.MonsterAttributeSet\"'") 1.0)
    (`KismetSystemLibrary.PrintString` "Phase2")))

(event `self.ReceiveBeginPlay`
  ;[1 1 1] BeginPlay
  (bind _asgscuser_widget (cast `GSCUserWidget` (`WidgetComponent.GetUserWidgetObject` (`self.HealthComponent`))))
  (`GSCUserWidget.InitializeWithAbilitySystem` _asgscuser_widget (`self.AbilitySystemComponent`)))

(event `self.GSCCoreComponent.OnDeath`
  ;[1 1 1] OnDeath
  (`self.StopAnimMontage` null)
  (`BrainComponent.StopLogic` (`AIController.BrainComponent` (`AIBlueprintHelperLibrary.GetAIController` self)) "Death")
  (`BlackboardComponent.SetValueAsEnum` (`AIController.Blackboard` (`AIBlueprintHelperLibrary.GetAIController` self)) (`self.State`) 3)
  (`|PlayMontage` (`self.Mesh`) "/Game/Monster/Darknessy/Anim/Montage/reBossDeathLong_Montage.reBossDeathLong_Montage" ; Death
    (:`then`
      _)
    (:`OnCompleted`
      _)
    (:`OnBlendOut`
      _)
    (:`OnInterrupted`
      _))
  (`KismetSystemLibrary.Delay` 2.0)
  (`self.K2_DestroyActor`)
  (`KismetSystemLibrary.PrintString` "Darknessy::Death"))

(fn `UpdateWalkSpeed`
  (params (MaxWalkSpeed :type "Float (single-precision)"))
  (set `CharacterMovementComponent.MaxWalkSpeed` MaxWalkSpeed (`self.CharacterMovement`)))

(fn `UserConstructionScript`
  (bind _customditithitactorcomponent (`self.CustomDitItHitActorComponent`))
  (`CustomDitItHitActorComponent.SetupVariables` _customditithitactorcomponent (`self.SkeletalMesh`) null)
  (`CustomDitItHitActorComponent.ToggleTraceCheck` _customditithitactorcomponent true))