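; Trigger volume that plays a background music track for a section of Stage 02 while the player is inside it.
; The audio component is stopped on BeginPlay.
; When an actor tagged Player begins overlapping the box collision the audio fades in, and when it ends overlap the audio fades out, both over a short fixed time.
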(event `self.ReceiveBeginPlay`
  (`AudioComponent.Stop` (`self.AudioComponent`)))

(event `self.BoxColl.OnComponentBeginOverlap`
  (params (OverlappedComponent :type "PrimitiveComponent Object Reference") (OtherActor :type "Actor Object Reference") (OtherComp :type "PrimitiveComponent Object Reference") (OtherBodyIndex :type Integer) (bFromSweep :type Boolean) (SweepResult :type "HitResult Structure (by ref)"))
  (if (`self.ActorHasTag` OtherActor "Player")
    (`AudioComponent.FadeIn` (`self.AudioComponent`) 0.5 1.0 0.0 "Linear")))

(event `self.BoxColl.OnComponentEndOverlap`
  (params (OverlappedComponent :type "PrimitiveComponent Object Reference") (OtherActor :type "Actor Object Reference") (OtherComp :type "PrimitiveComponent Object Reference") (OtherBodyIndex :type Integer))
  (if (`self.ActorHasTag` OtherActor "Player")
    (`AudioComponent.FadeOut` (`self.AudioComponent`) 0.5 0.0 "Linear")))

(fn `UserConstructionScript`)