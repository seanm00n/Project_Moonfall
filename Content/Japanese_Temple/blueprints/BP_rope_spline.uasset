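; Rope actor that builds its mesh along an editable spline in the construction script, with no runtime logic.
; Each span between spline points gets a collidable spline mesh following the point positions and tangents.
; Knot01, Knot02, RopeStart and RopeEnd flags add scaled, offset end pieces aligned to the first or last point's tangent.
; Both knot branches loop per segment, stacking identical pieces at the same endpoint.
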(fn `UserConstructionScript`
  (bind _spline (`self.Spline`))
  (bind _spline_2 (`self.Spline`))
  (bind _spline_3 (`self.Spline`))
  (bind _spline_4 (`self.Spline`))
  (bind (_location _tangent) (`SplineComponent.GetLocationAndTangentAtSplinePoint` (`self.Spline`) 0 "Local"))
  (bind (_location_2 _tangent_2) (`SplineComponent.GetLocationAndTangentAtSplinePoint` (`self.Spline`) 0 "Local"))
  (bind (_location_3 _tangent_3) (`SplineComponent.GetLocationAndTangentAtSplinePoint` _spline_4 (`SplineComponent.GetNumberOfSplinePoints` _spline_4) "Local"))
  (bind (_location_4 _tangent_4) (`SplineComponent.GetLocationAndTangentAtSplinePoint` _spline_3 (`SplineComponent.GetNumberOfSplinePoints` _spline_3) "Local"))
  (bind _returnvalue (`KismetMathLibrary.Conv_VectorToRotator` _tangent_2))
  (bind _returnvalue_2 (`KismetMathLibrary.Conv_VectorToRotator` _tangent))
  (bind _returnvalue_3 (`KismetMathLibrary.Conv_VectorToRotator` _tangent_3))
  (bind _returnvalue_4 (`KismetMathLibrary.Conv_VectorToRotator` _tangent_4))
  (`|ExecutionSequence`
    (:`then_0`
      (for _index (range (+ (- (`SplineComponent.GetNumberOfSplinePoints` (`self.Spline`)) 2) 1))
        (bind _returnvalue_5 (`AddComponent|NODE_AddSplineMeshComponent-0`))
        (`SplineMeshComponent.SetForwardAxis` _returnvalue_5 "X" true)
        (bind _returnvalue_6 (+ _index 1))
        (`SplineMeshComponent.SetStartAndEnd` _returnvalue_5 (`SplineComponent.GetLocationAtSplinePoint` _spline _index "Local") (`SplineComponent.GetTangentAtSplinePoint` _spline _index "Local") (`SplineComponent.GetLocationAtSplinePoint` _spline_2 _returnvalue_6 "Local") (`SplineComponent.GetTangentAtSplinePoint` _spline_2 _returnvalue_6 "Local") true)
        (`PrimitiveComponent.SetCollisionEnabled` _returnvalue_5 "QueryAndPhysics")))
    (:`then_1`
      (if (`self.knot_01`)
        (for _ (range (+ (- (`SplineComponent.GetNumberOfSplinePoints` (`self.Spline`)) 2) 1))
          (bind _returnvalue_7 (`AddComponent|NODE_AddSplineMeshComponent-1`))
          (`SceneComponent.K2_SetRelativeLocationAndRotation` _returnvalue_7 _location (select `ESplineMeshAxis` "X" :`X` _returnvalue_2 :`Y` (`KismetMathLibrary.MakeRotator` (+ (.roll _returnvalue_2) 90.0) (.pitch _returnvalue_2) (.yaw _returnvalue_2)) :`Z` (`KismetMathLibrary.MakeRotator` (.roll _returnvalue_2) (+ (.pitch _returnvalue_2) 90.0) (.yaw _returnvalue_2))) false false)
          (`SceneComponent.SetRelativeScale3D` _returnvalue_7 (0.3 1.0 1.0))
          (`SceneComponent.K2_AddLocalOffset` _returnvalue_7 (-20.0 0.0 0.0) false false)
          (`PrimitiveComponent.SetCollisionEnabled` _returnvalue_7 "QueryAndPhysics"))))
    (:`then_2`
      (if (`self.knot_02`)
        (for _ (range (+ (- (`SplineComponent.GetNumberOfSplinePoints` (`self.Spline`)) 2) 1))
          (bind _returnvalue_8 (`AddComponent|NODE_AddSplineMeshComponent-2`))
          (`SceneComponent.K2_SetRelativeLocationAndRotation` _returnvalue_8 _location_4 (select `ESplineMeshAxis` "X" :`X` _returnvalue_4 :`Y` (`KismetMathLibrary.MakeRotator` (+ (.roll _returnvalue_4) 90.0) (.pitch _returnvalue_4) (.yaw _returnvalue_4)) :`Z` (`KismetMathLibrary.MakeRotator` (.roll _returnvalue_4) (+ (.pitch _returnvalue_4) 90.0) (.yaw _returnvalue_4))) false false)
          (`SceneComponent.SetRelativeScale3D` _returnvalue_8 (0.3 1.0 1.0))
          (`SceneComponent.K2_AddLocalOffset` _returnvalue_8 (-20.0 0.0 0.0) false false)
          (`PrimitiveComponent.SetCollisionEnabled` _returnvalue_8 "QueryAndPhysics"))))
    (:`then_3`
      (if (`self.rope_end`)
        (bind _returnvalue_9 (`AddComponent|NODE_AddSplineMeshComponent-3`))
        (`SceneComponent.K2_SetRelativeLocationAndRotation` _returnvalue_9 _location_3 (select `ESplineMeshAxis` "X" :`X` _returnvalue_3 :`Y` (`KismetMathLibrary.MakeRotator` (+ (.roll _returnvalue_3) 90.0) (.pitch _returnvalue_3) (.yaw _returnvalue_3)) :`Z` (`KismetMathLibrary.MakeRotator` (.roll _returnvalue_3) (+ (.pitch _returnvalue_3) 90.0) (.yaw _returnvalue_3))) false false)
        (`SceneComponent.SetRelativeScale3D` _returnvalue_9 (0.3 1.0 1.0))
        (`SceneComponent.K2_AddLocalOffset` _returnvalue_9 (30.0 0.0 0.0) false false)
        (`SceneComponent.K2_AddLocalRotation` _returnvalue_9 (struct :`Yaw` 180.0) false false)
        (`PrimitiveComponent.SetCollisionEnabled` _returnvalue_9 "QueryAndPhysics")))
    (:`then_4`
      (if (`self.rope_start`)
        (bind _returnvalue_10 (`AddComponent|NODE_AddSplineMeshComponent-4`))
        (`SceneComponent.K2_SetRelativeLocationAndRotation` _returnvalue_10 _location_2 (select `ESplineMeshAxis` "X" :`X` _returnvalue :`Y` (`KismetMathLibrary.MakeRotator` (+ (.roll _returnvalue) 90.0) (.pitch _returnvalue) (.yaw _returnvalue)) :`Z` (`KismetMathLibrary.MakeRotator` (.roll _returnvalue) (+ (.pitch _returnvalue) 90.0) (.yaw _returnvalue))) false false)
        (`SceneComponent.SetRelativeScale3D` _returnvalue_10 (0.3 1.0 1.0))
        (`SceneComponent.K2_AddLocalOffset` _returnvalue_10 (-40.0 0.0 0.0) false false)
        (`SceneComponent.K2_AddLocalRotation` :`self` _returnvalue_10)
        (`PrimitiveComponent.SetCollisionEnabled` _returnvalue_10 "QueryAndPhysics")))))